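; Player character Blueprint for the RogueLike game, adding a health widget and a parry input on top of its action component.
; On BeginPlay it creates a MinionHealth_Widget attached to itself and adds it to the viewport.
; Pressing Parry starts the "Parry" action by name through ActionComp.
; A delayed Effect_Stunned add is left unconnected and never runs.
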(event `self.ReceiveBeginPlay`
  (bind _returnvalue (`|CreateWidget` "/Game/RogueLike/Blueprints/UI/MinionHealth_Widget.MinionHealth_Widget_C" null self))
  (`UserWidget.AddToViewport` _returnvalue 0))

(event `InputAction|Parry`
  (params (Key :type "Key Structure"))
  (:`Pressed`
    (`RLActionComponent.StartActionByName` (`self.ActionComp`) self "Parry")))

(fn `UserConstructionScript`)